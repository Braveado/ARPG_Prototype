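; AI controller for ARPG enemy characters that runs the EnemyAI_BT behavior tree and stores a spawn location on possession.
; AI perception updates whether the player character is visible in the Blackboard and caches the sensed character as the current target.
; Stagger, death and attack-combo checks write character and combat state enums to the Blackboard.
; Attack and state-reset events forward to the possessed enemy pawn.
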(event OnTargetPerceptionUpdated(AIPerception)
  (params (Actor :type Actor%20Object%20Reference) (Stimulus :type AI%20Stimulus%20Structure))
  ;[0.7109 1 0] AI Perception
  (bind _asarpg_character_bp (Utilities|Casting|CastToARPG_Character_BP Actor))
  (AI|Components|Blackboard|SetValueasBool (AI|GetBlackboard 0) (Utilities|Name|MakeLiteralName "CanSeeTarget") (.bsuccessfullysensed Stimulus))
  (if (.bsuccessfullysensed Stimulus)
    (Variables|Default|SetCurrentTarget _asarpg_character_bp)))

(event Custom|PawnAttack
  ;[1 0 0.6328] Attack
  (Default|Attack (Variables|Default|GetEnemyCharacterBP)))

(event Custom|CheckAttackCombo
  (bind _returnvalue (AI|GetBlackboard 0))
  (bind _returnvalue_2 (Utilities|Name|MakeLiteralName "CombatState"))
  ;[1 0 0.6328] Attack
  (if (> (Class|BlackboardComponent|GetValueasInt (AI|GetBlackboard 0) (Utilities|Name|MakeLiteralName "AttackCombo")) 0)
    (AI|Components|Blackboard|SetValueasEnum _returnvalue _returnvalue_2 (Utilities|Enum|LiteralenumAICombatState "NewEnumerator1"))
    (else
      (AI|Components|Blackboard|SetValueasEnum _returnvalue _returnvalue_2 (Utilities|Enum|LiteralenumAICombatState "NewEnumerator0")))))

(event Custom|PawnResetState
  ;[1 0 0.9609] Reset State
  (Default|ResetState (Variables|Default|GetEnemyCharacterBP)))

(event Custom|EndStagger
  ;[1 0.2109 0] Stagger
  (AI|Components|Blackboard|SetValueasEnum (AI|GetBlackboard 0) (Utilities|Name|MakeLiteralName "CharacterState") (Utilities|Enum|LiteralenumCharacterState "NewEnumerator0")))

(event Custom|StartStagger
  ;[1 0.2109 0] Stagger
  (AI|Components|Blackboard|SetValueasEnum (AI|GetBlackboard 0) (Utilities|Name|MakeLiteralName "CharacterState") (Utilities|Enum|LiteralenumCharacterState "NewEnumerator6")))

(event Custom|StartBehaviour
  ;[0.4766 1 0] Behaviour Switches
  (AI|RunBehaviorTree "/Game/ARPG_Prototype/AI/EnemyAI_BT.EnemyAI_BT")
  (AI|Components|Blackboard|SetValueasVector (AI|GetBlackboard 0) (Utilities|Name|MakeLiteralName "SpawnLocation") (Transformation|GetActorLocation)))

(event Custom|StopBehaviour
  ;[0.4766 1 0] Behaviour Switches
  (AI|Logic|StopLogic (Variables|Default|GetBrainComponent) ""))

(event EventPossess
  (params (PossessedPawn :type Pawn%20Object%20Reference))
  ;[0.6641 1 0] Event On Posses
  (bind _asenemy_ai_character_bp (Utilities|Casting|CastToEnemyAI_Character_BP PossessedPawn))
  (Variables|Default|SetEnemyCharacterBP _asenemy_ai_character_bp)
  (CallFunction|StartBehaviour))

(fn ConstructionScript)

(fn SetDead
  (AI|Components|Blackboard|SetValueasEnum (AI|GetBlackboard 0) (Utilities|Name|MakeLiteralName "CharacterState") (Utilities|Enum|LiteralenumCharacterState "NewEnumerator5")))