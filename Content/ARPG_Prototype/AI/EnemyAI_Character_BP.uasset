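; Enemy AI character for an ARPG prototype that picks a random mesh, fights with two alternating montage attacks and rewards XP and chance loot on death.
; Anim notifies toggle weapon overlaps and relay combo and stagger events to EnemyAI_Controller_BP.
; Weapon hits damage the player once per swing via DamagedActors, while secondary-weapon contact staggers the enemy.
; Received damage uses game-instance armor calculation, updates the HP bar, then staggers or kills.
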(event Custom|Attack
  ;[1 0.4453 0] Attack
  (Variables|State|SetCharacterState "NewEnumerator3")
  (switch int (Variables|Combat|GetAttackCount)
    (:0
      (Animation|PlayAnimMontage "/Game/ARPG_Prototype/Animations/ARPG_Attack01_RM_Montage.ARPG_Attack01_RM_Montage" 0.75 "None")
      (Variables|Combat|SetAttackCount 1))
    (:1
      (Animation|PlayAnimMontage "/Game/ARPG_Prototype/Animations/ARPG_Attack02_RM_Montage.ARPG_Attack02_RM_Montage" 0.75 "None")
      (Variables|Combat|SetAttackCount 0))))

(event Custom|EndStagger
  ;[0.4062 1 0] Stagger State
  (Variables|State|SetCharacterState "NewEnumerator0")
  (bind _asenemy_ai_controller_bp (Utilities|Casting|CastToEnemyAI_Controller_BP (Pawn|GetController)))
  (Default|EndStagger _asenemy_ai_controller_bp))

(event Custom|ControllerCheckAttackCombo
  ;[1 0.4453 0] Attack
  (bind _asenemy_ai_controller_bp (Utilities|Casting|CastToEnemyAI_Controller_BP (Pawn|GetController)))
  (Default|CheckAttackCombo _asenemy_ai_controller_bp))

(event Custom|ActivateWeaponCollision
  ;[1 0.2109 0] Weapon Collisions
  (Variables|/Script/Engine.PrimitiveComponent|SetbGenerateOverlapEvents (Variables|Default|GetWeaponCollision) true))

(event Custom|DeactivateWeaponCollision
  ;[1 0.2109 0] Weapon Collisions
  (Variables|/Script/Engine.PrimitiveComponent|SetbGenerateOverlapEvents (Variables|Default|GetWeaponCollision) false)
  (Utilities|Array|Clear (Variables|Combat|GetDamagedActors)))

(event Custom|ControllerStartStagger
  ;[0.4062 1 0] Stagger State
  (Variables|State|SetCharacterState "NewEnumerator6")
  (bind _asenemy_ai_controller_bp (Utilities|Casting|CastToEnemyAI_Controller_BP (Pawn|GetController)))
  (Default|StartStagger _asenemy_ai_controller_bp))

(event EventBeginPlay
  ;[0 1 0.2031] EventBeginPlay
  (CallFunction|SetRandomMesh)
  (CallFunction|InitializeEnemy))

(event Collision|EventActorBeginOverlap
  (params (OtherActor :type Actor%20Object%20Reference))
  ;[1 0 0.9609] Event Begin Overlap
  (bind _asarpg_character_bp (Utilities|Casting|CastToARPG_Character_BP OtherActor))
  (if (Class|PrimitiveComponent|IsOverlappingComponent (Variables|Default|GetWeaponCollision) (Variables|/Game/ARPG_Prototype/Blueprints/ARPG_Character_BP.ARPG_Character_BP_C|GetSecondaryWeaponCollision _asarpg_character_bp))
    (CallFunction|SetStagger)
    (elif (Collision|IsOverlappingActor (Variables|Default|GetWeaponCollision) _asarpg_character_bp :!class /Script/Engine.PrimitiveComponent)
      (bind _candamage (CallFunction|GetCanDamageActor _asarpg_character_bp))
      (if _candamage
        (Default|ReceiveDamage _asarpg_character_bp (Variables|Combat|GetDamage))
        (else
          (Development|PrintString "ALREADY DAMAGED" true true "(R=1.000000,G=0.025124,B=0.000000,A=1.000000)" 1e+01))))))

(fn ConstructionScript)

(fn InitializeEnemy
  (Variables|State|SetCurrentHP (Variables|State|GetMaxHP))
  (bind _asenemy_hp_wbp (Utilities|Casting|CastToEnemyHP_WBP (UserInterface|GetUserWidgetObject (Variables|Default|GetHPWidget))))
  (Variables|State|SetHPBar _asenemy_hp_wbp))

(fn ReceiveDamage
  (params (InputDamage :type Float%20%28single-precision%29))
  (if (Utilities|Enum|NotEqual(Enum) (Variables|State|GetCharacterState) "NewEnumerator5")
    (bind _asarpg_gi (Utilities|Casting|CastToARPG_GI (Game|GetGameInstance)))
    (bind _outputdamage (Default|CalculateDamage _asarpg_gi InputDamage (Variables|Combat|GetArmor)))
    (Variables|State|SetCurrentHP (Math|Float|Clamp(Float) (- (Variables|State|GetCurrentHP) _outputdamage) 0.0 (Variables|State|GetMaxHP)))
    (bind _returnvalue (Animation|GetCurrentMontage :!class /Script/Engine.Character))
    (Animation|StopAnimMontage _returnvalue)
    (CallFunction|ResetState)
    (if (<= (Variables|State|GetCurrentHP) 0.0)
      (Animation|PlayAnimMontage "/Game/ARPG_Prototype/Animations/ARPG_Death_Montage.ARPG_Death_Montage" 1.0 "None")
      (CallFunction|SetDead)
      (CallFunction|UpdateHPBar 1.0)
      (else
        (Animation|PlayAnimMontage "/Game/ARPG_Prototype/Animations/ARPG_Stagger_Montage.ARPG_Stagger_Montage" 1.0 "None")
        (CallFunction|UpdateHPBar 5.0)))))

(fn SetRandomMesh
  (bind _charactermeshes (Variables|Setup|GetCharacterMeshes))
  (Class|SkinnedMeshComponent|SetSkeletalMesh (Variables|Character|GetMesh) (Utilities|Array|Get(acopy) _charactermeshes (Math|Random|RandomIntegerinRange 0 (Utilities|Array|LastIndex _charactermeshes))) true))

(fn ResetState
  (Variables|State|SetCharacterState "NewEnumerator0")
  (Variables|Combat|SetAttackCount 0)
  (CallFunction|DeactivateWeaponCollision))

(fn SetDead
  (Variables|State|SetCharacterState "NewEnumerator5")
  (Collision|SetCollisionResponsetoChannel (Variables|Collision|GetCapsuleComponent) "ECC_Pawn" "ECR_Ignore")
  (bind _asenemy_ai_controller_bp (Utilities|Casting|CastToEnemyAI_Controller_BP (Pawn|GetController)))
  (Default|SetDead _asenemy_ai_controller_bp)
  (CallFunction|GiveXP)
  (CallFunction|CheckLootDrop)
  (Default|CallSignalDeath))

(fn SetStagger
  (bind _returnvalue (Animation|GetCurrentMontage :!class /Script/Engine.Character))
  (Animation|StopAnimMontage _returnvalue)
  (CallFunction|ResetState)
  (Animation|PlayAnimMontage "/Game/ARPG_Prototype/Animations/ARPG_Stagger_Montage.ARPG_Stagger_Montage" 1.0 "None"))

(fn UpdateHPBar
  (params (ShowSeconds :type Float%20%28single-precision%29))
  (Default|ShowHPBar (Variables|State|GetHPBar) (/ (Variables|State|GetCurrentHP) (Variables|State|GetMaxHP)) ShowSeconds))

(fn CheckLootDrop
  (if (<= (Math|Random|RandomFloat) (Variables|Progress|GetLootChance))
    (Game|SpawnActorfromClass "/Game/ARPG_Prototype/Items/LootActor.LootActor_C" (Transformation|GetActorTransform) "AdjustIfPossibleButAlwaysSpawn" 0 0)))

(fn GiveXP
  (bind _asarpg_character_bp (Utilities|Casting|CastToARPG_Character_BP (Game|Player|GetPlayerPawn 0)))
  (Default|GainEXP _asarpg_character_bp (Variables|Progress|GetRewardEXP)))

(fn GetCanDamageActor
  (params (InputActor :type Actor%20Object%20Reference))
  (if (not (Utilities|Array|ContainsItem (Variables|Combat|GetDamagedActors) InputActor))
    (Utilities|Array|Add (Variables|Combat|GetDamagedActors) InputActor)
    (return true)
    (else
      (return false))))