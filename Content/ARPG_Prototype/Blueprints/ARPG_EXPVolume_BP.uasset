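; A trigger volume Blueprint that grants experience to the player character while it stays inside.
; Beginning overlap with an ARPG_Character_BP stores the reference and starts a looping half-second timer that calls GainEXP with a fixed amount on each tick.
; Ending any overlap clears the stored character and invalidates the timer, without checking which actor left.
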(event Custom|GiveEXP
  (Default|GainEXP (Variables|Default|GetCharacterBP) 50))

(event Collision|EventActorBeginOverlap
  (params (OtherActor :type Actor%20Object%20Reference))
  (bind _asarpg_character_bp (Utilities|Casting|CastToARPG_Character_BP OtherActor))
  (Variables|Default|SetCharacterBP _asarpg_character_bp)
  (bind _returnvalue (Utilities|Time|SetTimerbyEvent (delegate Custom|GiveEXP) 0.5 true))
  (Variables|Default|SetTimerHandle _returnvalue))

(event Collision|EventActorEndOverlap
  (params (OtherActor :type Actor%20Object%20Reference))
  (Variables|Default|SetCharacterBP 0)
  (Utilities|Time|ClearandInvalidateTimerbyHandle (Variables|Default|GetTimerHandle)))

(fn ConstructionScript)