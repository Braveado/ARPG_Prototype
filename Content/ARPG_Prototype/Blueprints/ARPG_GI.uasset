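; ARPG game instance that saves, loads and deletes player EXP progress and picks the level to open on respawn.
; SaveGame writes current EXP and EXP currency into a cached ARPG_SaveGame object, then to the save slot.
; LoadGame returns the cached values, reading the slot only when no object is cached; DeleteSave clears just the slot.
; CheckPlayerRespawn opens the character test level if a save exists, otherwise the main menu.
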(fn SaveGame
  (params (InputCurrentEXP :type Integer) (InputEXPCurrency :type Integer))
  (Utilities|IsValid (Variables|Setup|GetSaveGameBP)
    (:Is%20Valid
      _)
    (:Is%20Not%20Valid
      (bind _returnvalue (SaveGame|CreateSaveGameObject "/Game/ARPG_Prototype/Blueprints/ARPG_SaveGame.ARPG_SaveGame_C"))
      (Variables|Setup|SetSaveGameBP _returnvalue)))
  (Utilities|FlowControl|Sequence
    (:then_0
      (Variables|/Game/ARPG_Prototype/Blueprints/ARPG_SaveGame.ARPG_SaveGame_C|SetEXPCurrency (Variables|Setup|GetSaveGameBP) InputEXPCurrency))
    (:then_1
      (Variables|/Game/ARPG_Prototype/Blueprints/ARPG_SaveGame.ARPG_SaveGame_C|SetCurrentEXP (Variables|Setup|GetSaveGameBP) InputCurrentEXP))
    (:then_2
      (SaveGame|SaveGametoSlot (Variables|Setup|GetSaveGameBP) (Variables|Setup|GetSaveSlotName)))))

(fn LoadGame
  (Utilities|IsValid (Variables|Setup|GetSaveGameBP)
    (:Is%20Valid
      _)
    (:Is%20Not%20Valid
      (bind _returnvalue (SaveGame|LoadGamefromSlot (Variables|Setup|GetSaveSlotName)))
      (bind _asarpg_save_game (Utilities|Casting|CastToARPG_SaveGame _returnvalue))
      (Variables|Setup|SetSaveGameBP _asarpg_save_game)))
  (return (Variables|/Game/ARPG_Prototype/Blueprints/ARPG_SaveGame.ARPG_SaveGame_C|GetCurrentEXP (Variables|Setup|GetSaveGameBP)) (Variables|/Game/ARPG_Prototype/Blueprints/ARPG_SaveGame.ARPG_SaveGame_C|GetEXPCurrency (Variables|Setup|GetSaveGameBP))))

(fn DeleteSave
  (bind _returnvalue (SaveGame|DoesSaveGameExist (Variables|Setup|GetSaveSlotName)))
  (if _returnvalue
    (SaveGame|DeleteGameinSlot (Variables|Setup|GetSaveSlotName))))

(fn CheckPlayerRespawn
  (bind _returnvalue (SaveGame|DoesSaveGameExist (Variables|Setup|GetSaveSlotName)))
  (if _returnvalue
    (Game|OpenLevel(byName) "ARPG_CharacterTest")
    (else
      (Game|OpenLevel(byName) "MainMenu"))))