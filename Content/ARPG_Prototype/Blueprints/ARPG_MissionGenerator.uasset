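; Mission generator that builds a randomized, linear tile layout for an ARPG mission, with length set by the game instance's MissionSize.
; TilesetSetup random-walks cardinal steps across a bounded grid without reusing cells, and MissionGeneration restarts it whenever the walk runs out of tries.
; TilesetGeneration picks start, end, straight or corner tiles and yaw from neighboring path directions, then spawns each as a streaming level instance centered around the origin.
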(event Custom|TilesetGeneration
  ;[1 0 0.3047] Tileset Generation
  (for (_array_element _array_index) (Variables|Tileset|GetTileGridLocations)
    (bind (_outputselectedtile _outputtilerotation) (CallFunction|GetNewSelectedTile _array_element _array_index))
    (bind _returnvalue (Class|LevelStreaming|CreateInstance _outputselectedtile (Utilities|String|ToString(Integer) _array_index)))
    (Variables|/Script/Engine.LevelStreaming|SetLevelTransform _returnvalue (Math|Transform|MakeTransform (Math|Vector|MakeVector (- (* (Math|Float|Truncate (.X (Math|Vector|BreakVector _array_element))) (Variables|Tileset|GetTileArea)) (/ (* (Variables|Tileset|GetGridSizeX) (Variables|Tileset|GetTileArea)) 2.0)) (- (* (Math|Float|Truncate (.Y (Math|Vector|BreakVector _array_element))) (Variables|Tileset|GetTileArea)) (/ (* (Variables|Tileset|GetGridSizeY) (Variables|Tileset|GetTileArea)) 2.0)) 0.0) _outputtilerotation))
    (Variables|/Script/Engine.LevelStreaming|SetbShouldBeLoaded _returnvalue true)
    (Variables|/Script/Engine.LevelStreaming|SetbShouldBeVisible _returnvalue true)))

(event Custom|TilesetSetup
  (bind _tilegridlocations (Variables|Tileset|GetTileGridLocations))
  (bind _tilegridlocations_2 (Variables|Tileset|GetTileGridLocations))
  ;[0 1 0.4375] Tileset Setup
  (Utilities|Array|Clear _tilegridlocations)
  (Utilities|Array|Add _tilegridlocations (Math|Vector|MakeVector (Math|Conversions|ToFloat(Integer) (Math|Random|RandomIntegerinRange 0 (- (Variables|Tileset|GetGridSizeX) 1))) (Math|Conversions|ToFloat(Integer) (Math|Random|RandomIntegerinRange 0 (- (Variables|Tileset|GetGridSizeY) 1))) 0.0)) ; Add starting tile
  (Variables|Tileset|SetGenerationFailed false)
  (CallFunction|GetTileAmountRange)
  (Utilities|FlowControl|ForLoopwithBreak 1 (- (Math|Random|RandomIntegerinRange (Variables|Tileset|GetMinTiles) (Variables|Tileset|GetMaxTiles)) 1) :!label _label
    (:LoopBody
      (bind (_outputlocation _outputfail) (CallFunction|GetNewTileGridLocation _tilegridlocations_2))
      (if _outputfail
        (Variables|Tileset|SetGenerationFailed true)
        (goto _label Break)
        (else
          (Utilities|Array|Add _tilegridlocations_2 _outputlocation))))))

(event Custom|MissionGeneration
  ;[0.4531 0 1] Mission Generation
  (CallFunction|TilesetSetup :!label _label)
  (if (Variables|Tileset|GetGenerationFailed)
    (goto _label)
    (else
      (CallFunction|TilesetGeneration))))

(fn ConstructionScript)

(fn GetNewTileGridLocation
  (params (InputLocations :type Array%20of%20Vectors))
  (LocalVariables|SetLastLocation (Utilities|Array|Get(acopy) InputLocations (- (Utilities|Array|Length InputLocations) 1)))
  (while (and (LocalVariables|GetCheckNewLocation) (not (LocalVariables|GetMaxTries)))
    (LocalVariables|SetNewLocation (LocalVariables|GetLastLocation))
    (switch int (Math|Random|RandomInteger 4) ; Move in a cardinal direction
      (:0
        (LocalVariables|SetNewLocation (Math|Vector|MakeVector (+ (.x (LocalVariables|GetNewLocation)) 1.0) (.y (LocalVariables|GetNewLocation)) (.z (LocalVariables|GetNewLocation)))))
      (:1
        (LocalVariables|SetNewLocation (Math|Vector|MakeVector (+ (.x (LocalVariables|GetNewLocation)) -1.0) (.y (LocalVariables|GetNewLocation)) (.z (LocalVariables|GetNewLocation)))))
      (:2
        (LocalVariables|SetNewLocation (Math|Vector|MakeVector (.x (LocalVariables|GetNewLocation)) (+ (.y (LocalVariables|GetNewLocation)) 1.0) (.z (LocalVariables|GetNewLocation)))))
      (:3
        (LocalVariables|SetNewLocation (Math|Vector|MakeVector (.x (LocalVariables|GetNewLocation)) (+ (.y (LocalVariables|GetNewLocation)) -1.0) (.z (LocalVariables|GetNewLocation))))))
    (LocalVariables|SetNewLocation (Math|Vector|MakeVector (Math|Float|Clamp(Float) (.x (LocalVariables|GetNewLocation)) 0.0 (Math|Conversions|ToFloat(Integer) (- (Variables|Tileset|GetGridSizeX) 1))) (Math|Float|Clamp(Float) (.y (LocalVariables|GetNewLocation)) 0.0 (Math|Conversions|ToFloat(Integer) (- (Variables|Tileset|GetGridSizeY) 1))) 0.0)) ; Clamp location to grid
    (bind _array_element (Utilities|Array|ForEachLoopwithBreak InputLocations :!label _label) ; Prevent used locations
      (:LoopBody
        (if (Math|Vector|Equal(Vector) _array_element (LocalVariables|GetNewLocation) 0.0001)
          (Math|Integer|IncrementInt (LocalVariables|GetNewLocationTries)
            (:%20%20
              (LocalVariables|SetLocationCheckBreak true)
              (goto _label Break)))))
      (:Completed
        (if (LocalVariables|GetLocationCheckBreak)
          (LocalVariables|SetLocationCheckBreak false)
          (if (>= (LocalVariables|GetNewLocationTries) (LocalVariables|GetMaxLocationTries))
            (LocalVariables|SetMaxTries true))
          (else
            (LocalVariables|SetCheckNewLocation false))))))
  (return (LocalVariables|GetNewLocation) (LocalVariables|GetMaxTries)))

(fn GetNewSelectedTile
  (params (InputTileLocation :type Vector) (InputTileIndex :type Integer))
  (LocalVariables|SetTileLocation InputTileLocation)
  (LocalVariables|SetTileIndex InputTileIndex)
  (Utilities|FlowControl|Sequence
    (:then_0
      (if (<= (+ (LocalVariables|GetTileIndex) 1) (Utilities|Array|LastIndex (Variables|Tileset|GetTileGridLocations))) ; Set next room
        (LocalVariables|SetNextTileLocation (Utilities|Array|Get(acopy) (Variables|Tileset|GetTileGridLocations) (+ (LocalVariables|GetTileIndex) 1)))
        (if (== (.x (LocalVariables|GetTileLocation)) (.x (LocalVariables|GetNextTileLocation)))
          (if (> (.y (LocalVariables|GetTileLocation)) (.y (LocalVariables|GetNextTileLocation)))
            (LocalVariables|SetNextTileDirection "NewEnumerator1")
            (else
              (LocalVariables|SetNextTileDirection "NewEnumerator2")))
          (elif (< (.x (LocalVariables|GetTileLocation)) (.x (LocalVariables|GetNextTileLocation)))
            (LocalVariables|SetNextTileDirection "NewEnumerator3")
            (else
              (LocalVariables|SetNextTileDirection "NewEnumerator4"))))))
    (:then_1
      (if (>= (- (LocalVariables|GetTileIndex) 1) 0) ; Set prev room
        (LocalVariables|SetPrevTileLocation (Utilities|Array|Get(acopy) (Variables|Tileset|GetTileGridLocations) (- (LocalVariables|GetTileIndex) 1)))
        (if (== (.x (LocalVariables|GetTileLocation)) (.x (LocalVariables|GetPrevTileLocation)))
          (if (> (.y (LocalVariables|GetTileLocation)) (.y (LocalVariables|GetPrevTileLocation)))
            (LocalVariables|SetPrevTileDirection "NewEnumerator1")
            (else
              (LocalVariables|SetPrevTileDirection "NewEnumerator2")))
          (elif (< (.x (LocalVariables|GetTileLocation)) (.x (LocalVariables|GetPrevTileLocation)))
            (LocalVariables|SetPrevTileDirection "NewEnumerator3")
            (else
              (LocalVariables|SetPrevTileDirection "NewEnumerator4"))))))
    (:then_2
      (if (and (Utilities|Enum|NotEqual(Enum) (LocalVariables|GetNextTileDirection) "NewEnumerator0") (Utilities|Enum|NotEqual(Enum) (LocalVariables|GetPrevTileDirection) "NewEnumerator0")) ; Set middle room
        (LocalVariables|SetTileSelectionIndex 0)
        (if (or (and (Utilities|Enum|Equal(Enum) (LocalVariables|GetNextTileDirection) "NewEnumerator1") (Utilities|Enum|Equal(Enum) (LocalVariables|GetPrevTileDirection) "NewEnumerator2")) (and (Utilities|Enum|Equal(Enum) (LocalVariables|GetNextTileDirection) "NewEnumerator2") (Utilities|Enum|Equal(Enum) (LocalVariables|GetPrevTileDirection) "NewEnumerator1")))
          (LocalVariables|SetTileSelectionIndex 2)
          (LocalVariables|SetSelectedTileRotation 9e+01)
          (elif (or (and (Utilities|Enum|Equal(Enum) (LocalVariables|GetNextTileDirection) "NewEnumerator3") (Utilities|Enum|Equal(Enum) (LocalVariables|GetPrevTileDirection) "NewEnumerator4")) (and (Utilities|Enum|Equal(Enum) (LocalVariables|GetNextTileDirection) "NewEnumerator4") (Utilities|Enum|Equal(Enum) (LocalVariables|GetPrevTileDirection) "NewEnumerator3")))
            (LocalVariables|SetTileSelectionIndex 2)
            (LocalVariables|SetSelectedTileRotation 0.0)
            (elif (or (and (Utilities|Enum|Equal(Enum) (LocalVariables|GetNextTileDirection) "NewEnumerator3") (Utilities|Enum|Equal(Enum) (LocalVariables|GetPrevTileDirection) "NewEnumerator2")) (and (Utilities|Enum|Equal(Enum) (LocalVariables|GetNextTileDirection) "NewEnumerator2") (Utilities|Enum|Equal(Enum) (LocalVariables|GetPrevTileDirection) "NewEnumerator3")))
              (LocalVariables|SetTileSelectionIndex 3)
              (LocalVariables|SetSelectedTileRotation 0.0)
              (elif (or (and (Utilities|Enum|Equal(Enum) (LocalVariables|GetNextTileDirection) "NewEnumerator2") (Utilities|Enum|Equal(Enum) (LocalVariables|GetPrevTileDirection) "NewEnumerator4")) (and (Utilities|Enum|Equal(Enum) (LocalVariables|GetNextTileDirection) "NewEnumerator4") (Utilities|Enum|Equal(Enum) (LocalVariables|GetPrevTileDirection) "NewEnumerator2")))
                (LocalVariables|SetTileSelectionIndex 3)
                (LocalVariables|SetSelectedTileRotation 9e+01)
                (elif (or (and (Utilities|Enum|Equal(Enum) (LocalVariables|GetNextTileDirection) "NewEnumerator4") (Utilities|Enum|Equal(Enum) (LocalVariables|GetPrevTileDirection) "NewEnumerator1")) (and (Utilities|Enum|Equal(Enum) (LocalVariables|GetNextTileDirection) "NewEnumerator1") (Utilities|Enum|Equal(Enum) (LocalVariables|GetPrevTileDirection) "NewEnumerator4")))
                  (LocalVariables|SetTileSelectionIndex 3)
                  (LocalVariables|SetSelectedTileRotation 1.8e+02)
                  (elif (or (and (Utilities|Enum|Equal(Enum) (LocalVariables|GetNextTileDirection) "NewEnumerator1") (Utilities|Enum|Equal(Enum) (LocalVariables|GetPrevTileDirection) "NewEnumerator3")) (and (Utilities|Enum|Equal(Enum) (LocalVariables|GetNextTileDirection) "NewEnumerator3") (Utilities|Enum|Equal(Enum) (LocalVariables|GetPrevTileDirection) "NewEnumerator1")))
                    (LocalVariables|SetTileSelectionIndex 3)
                    (LocalVariables|SetSelectedTileRotation 2.7e+02)))))))
        (elif (and (Utilities|Enum|NotEqual(Enum) (LocalVariables|GetNextTileDirection) "NewEnumerator0") (Utilities|Enum|Equal(Enum) (LocalVariables|GetPrevTileDirection) "NewEnumerator0")) ; Set first room
          (LocalVariables|SetTileSelectionIndex 4)
          (switch Utilities|FlowControl|Switch|SwitchonTileDirection (LocalVariables|GetNextTileDirection)
            (:NewEnumerator1
              (LocalVariables|SetSelectedTileRotation 2.7e+02))
            (:NewEnumerator2
              (LocalVariables|SetSelectedTileRotation 9e+01))
            (:NewEnumerator3
              (LocalVariables|SetSelectedTileRotation 0.0))
            (:NewEnumerator4
              (LocalVariables|SetSelectedTileRotation 1.8e+02)))
          (elif (and (Utilities|Enum|Equal(Enum) (LocalVariables|GetNextTileDirection) "NewEnumerator0") (Utilities|Enum|NotEqual(Enum) (LocalVariables|GetPrevTileDirection) "NewEnumerator0")) ; Set last room
            (LocalVariables|SetTileSelectionIndex 1)
            (switch Utilities|FlowControl|Switch|SwitchonTileDirection (LocalVariables|GetPrevTileDirection)
              (:NewEnumerator1
                (LocalVariables|SetSelectedTileRotation 2.7e+02))
              (:NewEnumerator2
                (LocalVariables|SetSelectedTileRotation 9e+01))
              (:NewEnumerator3
                (LocalVariables|SetSelectedTileRotation 0.0))
              (:NewEnumerator4
                (LocalVariables|SetSelectedTileRotation 1.8e+02)))))))
    (:then_3
      (return (Class|GameplayStatics|GetStreamingLevel (Utilities|Array|Get(acopy) (Variables|Tileset|GetTiles) (LocalVariables|GetTileSelectionIndex))) (Math|Rotator|MakeRotator 0.0 0.0 (LocalVariables|GetSelectedTileRotation))))))

(fn GetTileAmountRange
  (bind _asarpg_gi (Utilities|Casting|CastToARPG_GI (Game|GetGameInstance)))
  (switch Utilities|FlowControl|Switch|SwitchonMissionSize (Variables|/Game/ARPG_Prototype/Blueprints/ARPG_GI.ARPG_GI_C|GetMissionSize _asarpg_gi)
    (:NewEnumerator1
      (Variables|Tileset|SetMinTiles 3)
      (Variables|Tileset|SetMaxTiles 5))
    (:NewEnumerator2
      (Variables|Tileset|SetMinTiles 5)
      (Variables|Tileset|SetMaxTiles 7))
    (:NewEnumerator3
      (Variables|Tileset|SetMinTiles 7)
      (Variables|Tileset|SetMaxTiles 9))))