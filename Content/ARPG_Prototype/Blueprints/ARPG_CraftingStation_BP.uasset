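; Crafting station actor for the ARPG prototype that accepts player input while the character overlaps it.
; Use opens a new inventory widget and a crafting widget linked to it, shows the cursor and disables pawn input.
; Return returns items left in the two craft slots to the character's inventory, closes both widgets and restores game input.
; It also toggles off the character's own inventory screen if that is open.
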(event Collision|EventActorBeginOverlap
  (params (OtherActor :type Actor%20Object%20Reference))
  (Utilities|Casting|CastToARPG_Character_BP OtherActor)
  (Input|EnableInput (Game|GetPlayerController 0)))

(event Collision|EventActorEndOverlap
  (params (OtherActor :type Actor%20Object%20Reference))
  (Utilities|Casting|CastToARPG_Character_BP OtherActor)
  (Input|DisableInput (Game|GetPlayerController 0)))

(event Input|ActionEvents|InputActionUse
  (params (Key :type Key%20Structure :default "None"))
  (bind _returnvalue (Game|GetPlayerController 0))
  (:Pressed
    (Utilities|IsValid (Variables|Default|GetCraftingStationWBP)
      (:Is%20Valid
        (if (not (UserInterface|Viewport|IsinViewport (Variables|Default|GetCraftingStationWBP)))
          (Utilities|FlowControl|Sequence :!label _label
            (:then_0
              (bind _returnvalue_2 (UserInterface|CreateWidget "/Game/ARPG_Prototype/UI/Inventory/Inventory_WBP.Inventory_WBP_C"))
              (bind _output_get (Variables|Default|SetInventoryWBP _returnvalue_2))
              (UserInterface|Viewport|AddtoViewport _output_get 0))
            (:then_1
              (bind _returnvalue_3 (UserInterface|CreateWidget "/Game/ARPG_Prototype/UI/Crafting/CraftingStationWBP.CraftingStationWBP_C"))
              (bind _output_get_2 (Variables|Default|SetCraftingStationWBP _returnvalue_3))
              (Variables|/Game/ARPG_Prototype/UI/Crafting/CraftingStationWBP.CraftingStationWBP_C|SetInventoryWBP _output_get_2 (Variables|Default|GetInventoryWBP))
              (UserInterface|Viewport|AddtoViewport _output_get_2 0)
              (Input|SetInputModeGameandUI _returnvalue 0 "DoNotLock" true)
              (Variables|/Script/Engine.PlayerController|SetbShowMouseCursor _returnvalue true)
              (Input|DisableInput (Pawn|GetControlledPawn _returnvalue) _returnvalue)))))
      (:Is%20Not%20Valid
        (goto _label)))))

(event Input|ActionEvents|InputActionReturn
  (params (Key :type Key%20Structure :default "None"))
  (bind _returnvalue (Game|GetPlayerCharacter 0))
  (bind _returnvalue_2 (Game|GetPlayerController 0))
  (bind _craftingstationwbp (Variables|Default|GetCraftingStationWBP))
  (bind _craftingstationwbp_2 (Variables|Default|GetCraftingStationWBP))
  (bind _craftingstationwbp_3 (Variables|Default|GetCraftingStationWBP))
  (bind _inventorywbp (Variables|Default|GetInventoryWBP))
  (bind _asarpg_character_bp (Utilities|Casting|CastToARPG_Character_BP _returnvalue))
  (bind _inventory (Variables|/Game/ARPG_Prototype/Blueprints/ARPG_Character_BP.ARPG_Character_BP_C|GetInventory _asarpg_character_bp))
  (:Pressed
    (Utilities|FlowControl|Sequence
      (:then_0
        (Utilities|IsValid _inventorywbp
          (:Is%20Valid
            (if (UserInterface|Viewport|IsinViewport _inventorywbp)
              (Widget|RemovefromParent (Variables|Default|GetInventoryWBP))))))
      (:then_1
        (Utilities|IsValid _craftingstationwbp_3
          (:Is%20Valid
            (if (UserInterface|Viewport|IsinViewport _craftingstationwbp_3)
              (Utilities|FlowControl|Sequence
                (:then_0
                  (if (not (Utilities|Enum|Equal(Enum) (.Type (Utilities|Struct|BreakItemData (Variables|/Game/ARPG_Prototype/UI/Inventory/GearSlot_WBP.GearSlot_WBP_C|GetItemData (Variables|/Game/ARPG_Prototype/UI/Crafting/CraftingStationWBP.CraftingStationWBP_C|GetCraftSlotItem _craftingstationwbp)))) "NewEnumerator0"))
                    (Default|AddInventoryItem _inventory (Variables|/Game/ARPG_Prototype/UI/Inventory/GearSlot_WBP.GearSlot_WBP_C|GetItemData (Variables|/Game/ARPG_Prototype/UI/Crafting/CraftingStationWBP.CraftingStationWBP_C|GetCraftSlotItem _craftingstationwbp_2)))))
                (:then_1
                  (if (not (Utilities|Enum|Equal(Enum) (.Type (Utilities|Struct|BreakItemData (Variables|/Game/ARPG_Prototype/UI/Inventory/GearSlot_WBP.GearSlot_WBP_C|GetItemData (Variables|/Game/ARPG_Prototype/UI/Crafting/CraftingStationWBP.CraftingStationWBP_C|GetCraftSlotMod _craftingstationwbp)))) "NewEnumerator0"))
                    (Default|AddInventoryItem _inventory (Variables|/Game/ARPG_Prototype/UI/Inventory/GearSlot_WBP.GearSlot_WBP_C|GetItemData (Variables|/Game/ARPG_Prototype/UI/Crafting/CraftingStationWBP.CraftingStationWBP_C|GetCraftSlotMod _craftingstationwbp_2)))))
                (:then_2
                  (Widget|RemovefromParent (Variables|Default|GetCraftingStationWBP))
                  (Input|SetInputModeGameOnly _returnvalue_2)
                  (Variables|/Script/Engine.PlayerController|SetbShowMouseCursor _returnvalue_2 false)
                  (Input|EnableInput (Pawn|GetControlledPawn _returnvalue_2) _returnvalue_2)
                  (bind _asarpg_character_bp_2 (Utilities|Casting|CastToARPG_Character_BP (Game|GetPlayerCharacter 0)))
                  (Utilities|IsValid (Variables|/Game/ARPG_Prototype/Blueprints/ARPG_Character_BP.ARPG_Character_BP_C|GetInventoryWBP _asarpg_character_bp_2)
                    (:Is%20Valid
                      (if (UserInterface|Viewport|IsinViewport (Variables|/Game/ARPG_Prototype/Blueprints/ARPG_Character_BP.ARPG_Character_BP_C|GetInventoryWBP _asarpg_character_bp_2))
                        (Default|InventoryFlipFlop _asarpg_character_bp_2)))))))))))))

(fn ConstructionScript)