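; Interactable skills station actor that opens the skills station widget for the player.
; Overlap with the ARPG character enables the station's own input, and ending overlap disables it.
; Use lazily creates and caches the widget, shows it with cursor and Game-and-UI input, and disables pawn input.
; Return removes the widget and restores game-only input, hidden cursor and pawn control.
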(event Collision|EventActorBeginOverlap
  (params (OtherActor :type Actor%20Object%20Reference))
  (Utilities|Casting|CastToARPG_Character_BP OtherActor)
  (Input|EnableInput (Game|GetPlayerController 0)))

(event Collision|EventActorEndOverlap
  (params (OtherActor :type Actor%20Object%20Reference))
  (Utilities|Casting|CastToARPG_Character_BP OtherActor)
  (Input|DisableInput (Game|GetPlayerController 0)))

(event Input|ActionEvents|InputActionUse
  (params (Key :type Key%20Structure :default "None"))
  (bind _returnvalue (Game|GetPlayerController 0))
  (:Pressed
    (Utilities|IsValid (Variables|Default|GetStationWBP)
      (:Is%20Valid
        (if (not (UserInterface|Viewport|IsinViewport (Variables|Default|GetStationWBP)))
          (UserInterface|Viewport|AddtoViewport (stale _output_get) 0 :!label _label)
          (Input|SetInputModeGameandUI _returnvalue 0 "DoNotLock" true)
          (Variables|/Script/Engine.PlayerController|SetbShowMouseCursor _returnvalue true)
          (Input|DisableInput (Pawn|GetControlledPawn _returnvalue) _returnvalue)))
      (:Is%20Not%20Valid
        (bind _returnvalue_2 (UserInterface|CreateWidget "/Game/ARPG_Prototype/UI/SkillsSystem/ARPG_SkillsStation_WBP.ARPG_SkillsStation_WBP_C"))
        (bind _output_get (Variables|Default|SetStationWBP _returnvalue_2))
        (goto _label)))))

(event Input|ActionEvents|InputActionReturn
  (params (Key :type Key%20Structure :default "None"))
  (bind _returnvalue (Game|GetPlayerController 0))
  (bind _stationwbp (Variables|Default|GetStationWBP))
  (:Pressed
    (Utilities|IsValid _stationwbp
      (:Is%20Valid
        (if (UserInterface|Viewport|IsinViewport _stationwbp)
          (Widget|RemovefromParent _stationwbp)
          (Input|SetInputModeGameOnly _returnvalue)
          (Variables|/Script/Engine.PlayerController|SetbShowMouseCursor _returnvalue false)
          (Input|EnableInput (Pawn|GetControlledPawn _returnvalue) _returnvalue))))))

(fn ConstructionScript)