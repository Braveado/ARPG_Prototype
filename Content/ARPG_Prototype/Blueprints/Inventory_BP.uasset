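; Inventory Blueprint for the ARPG prototype that stores a capped item list and the equipped gear slots.
; Items are added only while space remains, and removed or overwritten by index after validity checks.
; Gear functions set, fetch or test emptiness of slots, routing by item type and armor or weapon subtype to head, chest, arms, legs, primary (sword) or secondary (shield).
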(event Custom|AddInventoryItem
  (params (InputItem :type Item%20Data%20Structure))
  (bind _availablespace (CallFunction|CheckAvailableSpace))
  (if _availablespace
    (Utilities|Array|Add (Variables|Inventory|GetInventoryItems) InputItem)))

(event Custom|SetGearSlotItem
  (params (InputItem :type Item%20Data%20Structure))
  (bind (_type _name _thumbnail _armordata _weapondata) (Utilities|Struct|BreakItemData InputItem))
  (switch Utilities|FlowControl|Switch|SwitchonItemType _type
    (:NewEnumerator1
      (switch Utilities|FlowControl|Switch|SwitchonArmorType (.Type (Utilities|Struct|BreakArmorData _armordata))
        (:NewEnumerator1
          (Variables|GearSlots|SetHeadSlot InputItem))
        (:NewEnumerator2
          (Variables|GearSlots|SetChestSlot InputItem))
        (:NewEnumerator3
          (Variables|GearSlots|SetArmsSlot InputItem))
        (:NewEnumerator4
          (Variables|GearSlots|SetLegsSlot InputItem))))
    (:NewEnumerator3
      (switch Utilities|FlowControl|Switch|SwitchonWeaponType (.Tyoe (Utilities|Struct|BreakWeaponData _weapondata))
        (:NewEnumerator1
          (Variables|GearSlots|SetPrimaryWeaponSlot InputItem))
        (:NewEnumerator2
          (Variables|GearSlots|SetSecondaryWeaponSlot InputItem))))))

(event Custom|RemoveInventoryItem
  (params (ItenIndex :type Integer))
  (bind _inventoryitems (Variables|Inventory|GetInventoryItems))
  (if (Utilities|Array|IsValidIndex _inventoryitems ItenIndex)
    (Utilities|Array|RemoveIndex _inventoryitems ItenIndex)))

(event EventBeginPlay)

(event EventTick
  (params (DeltaSeconds :type Float%20%28single-precision%29)))

(fn CheckEmptyGearSlot
  (params (InputItem :type Item%20Data%20Structure))
  (bind (_type _name _thumbnail _armordata _weapondata) (Utilities|Struct|BreakItemData InputItem))
  (Utilities|FlowControl|Sequence
    (:then_0
      (switch Utilities|FlowControl|Switch|SwitchonItemType _type
        (:NewEnumerator1
          (switch Utilities|FlowControl|Switch|SwitchonArmorType (.Type (Utilities|Struct|BreakArmorData _armordata))
            (:NewEnumerator1
              (LocalVariables|SetOutput (Utilities|Enum|Equal(Enum) (.Type (Utilities|Struct|BreakItemData (Variables|GearSlots|GetHeadSlot))) "NewEnumerator0")))
            (:NewEnumerator2
              (LocalVariables|SetOutput (Utilities|Enum|Equal(Enum) (.Type (Utilities|Struct|BreakItemData (Variables|GearSlots|GetChestSlot))) "NewEnumerator0")))
            (:NewEnumerator3
              (LocalVariables|SetOutput (Utilities|Enum|Equal(Enum) (.Type (Utilities|Struct|BreakItemData (Variables|GearSlots|GetArmsSlot))) "NewEnumerator0")))
            (:NewEnumerator4
              (LocalVariables|SetOutput (Utilities|Enum|Equal(Enum) (.Type (Utilities|Struct|BreakItemData (Variables|GearSlots|GetLegsSlot))) "NewEnumerator0")))))
        (:NewEnumerator3
          (switch Utilities|FlowControl|Switch|SwitchonWeaponType (.Tyoe (Utilities|Struct|BreakWeaponData _weapondata))
            (:NewEnumerator1
              (LocalVariables|SetOutput (Utilities|Enum|Equal(Enum) (.Type (Utilities|Struct|BreakItemData (Variables|GearSlots|GetPrimaryWeaponSlot))) "NewEnumerator0")))
            (:NewEnumerator2
              (LocalVariables|SetOutput (Utilities|Enum|Equal(Enum) (.Type (Utilities|Struct|BreakItemData (Variables|GearSlots|GetSecondaryWeaponSlot))) "NewEnumerator0")))))))
    (:then_1
      (return (LocalVariables|GetOutput)))))

(fn CheckAvailableSpace
  (return (< (Utilities|Array|Length (Variables|Inventory|GetInventoryItems)) (Variables|Inventory|GetMaxInventorySpace))))

(fn GetGearSlotItem
  (params (ItemInput :type Item%20Data%20Structure))
  (bind (_type _name _thumbnail _armordata _weapondata) (Utilities|Struct|BreakItemData ItemInput))
  (Utilities|FlowControl|Sequence
    (:then_0
      (switch Utilities|FlowControl|Switch|SwitchonItemType _type
        (:NewEnumerator1
          (switch Utilities|FlowControl|Switch|SwitchonArmorType (.Type (Utilities|Struct|BreakArmorData _armordata))
            (:NewEnumerator1
              (LocalVariables|SetLocalItem (Variables|GearSlots|GetHeadSlot)))
            (:NewEnumerator2
              (LocalVariables|SetLocalItem (Variables|GearSlots|GetChestSlot)))
            (:NewEnumerator3
              (LocalVariables|SetLocalItem (Variables|GearSlots|GetArmsSlot)))
            (:NewEnumerator4
              (LocalVariables|SetLocalItem (Variables|GearSlots|GetLegsSlot)))))
        (:NewEnumerator3
          (switch Utilities|FlowControl|Switch|SwitchonWeaponType (.Tyoe (Utilities|Struct|BreakWeaponData _weapondata))
            (:NewEnumerator1
              (LocalVariables|SetLocalItem (Variables|GearSlots|GetPrimaryWeaponSlot)))
            (:NewEnumerator2
              (LocalVariables|SetLocalItem (Variables|GearSlots|GetSecondaryWeaponSlot)))))))
    (:then_1
      (return (LocalVariables|GetLocalItem)))))

(fn SetInventoryItem
  (params (ItemIndex :type Integer) (InputItem :type Item%20Data%20Structure))
  (bind _inventoryitems (Variables|Inventory|GetInventoryItems))
  (if (Utilities|Array|IsValidIndex _inventoryitems ItemIndex)
    (Utilities|Array|SetArrayElem _inventoryitems ItemIndex InputItem)))