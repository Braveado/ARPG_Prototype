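; ARPG map station actor that lets the player open a map station widget while standing in its overlap area.
; Overlap by the ARPG character toggles actor input and active particles, and prints a key hint on entry.
; Use lazily creates and caches the widget, shows it with cursor and UI focus, and disables pawn input.
; Return removes the widget and restores game-only input and pawn control.
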(event Collision|EventActorBeginOverlap
  (params (OtherActor :type Actor%20Object%20Reference))
  (Utilities|Casting|CastToARPG_Character_BP OtherActor)
  (Input|EnableInput (Game|GetPlayerController 0))
  (Components|Activation|Activate (Variables|Default|GetActive_Particles) false)
  (Development|PrintString "OPEN: X, CLOSE: ESC"))

(event Collision|EventActorEndOverlap
  (params (OtherActor :type Actor%20Object%20Reference))
  (Utilities|Casting|CastToARPG_Character_BP OtherActor)
  (Input|DisableInput (Game|GetPlayerController 0))
  (Components|Activation|Deactivate (Variables|Default|GetActive_Particles)))

(event Input|ActionEvents|InputActionUse
  (params (Key :type Key%20Structure :default "None"))
  (bind _returnvalue (Game|GetPlayerController 0))
  (:Pressed
    (Utilities|IsValid (Variables|Default|GetStationWBP)
      (:Is%20Valid
        (if (not (UserInterface|Viewport|IsinViewport (Variables|Default|GetStationWBP)))
          (UserInterface|Viewport|AddtoViewport (stale _output_get) 0 :!label _label)
          (Input|SetInputModeGameandUI _returnvalue (Variables|Default|GetStationWBP) "DoNotLock" true)
          (Variables|/Script/Engine.PlayerController|SetbShowMouseCursor _returnvalue true)
          (Input|DisableInput (Pawn|GetControlledPawn _returnvalue) _returnvalue)))
      (:Is%20Not%20Valid
        (bind _returnvalue_2 (UserInterface|CreateWidget "/Game/ARPG_Prototype/UI/MapSystem/ARPG_MapStation_WBP.ARPG_MapStation_WBP_C"))
        (bind _output_get (Variables|Default|SetStationWBP _returnvalue_2))
        (goto _label)))))

(event Input|ActionEvents|InputActionReturn
  (params (Key :type Key%20Structure :default "None"))
  (bind _returnvalue (Game|GetPlayerController 0))
  (:Pressed
    (Widget|RemovefromParent (Variables|Default|GetStationWBP))
    (Input|SetInputModeGameOnly _returnvalue)
    (Variables|/Script/Engine.PlayerController|SetbShowMouseCursor _returnvalue false)
    (Input|EnableInput (Pawn|GetControlledPawn _returnvalue) _returnvalue)))

(fn ConstructionScript)